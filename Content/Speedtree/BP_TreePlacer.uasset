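; Tree placer that scatters randomly scaled and rotated tree meshes over a landscape at construction time, along with monster spawners.
; Random downward traces within XY bounds keep landscape hits that pass slope, minimum elevation and spacing checks.
; Each tree gets a repelling sphere component with an optional debug mesh.
; Tree locations also receive monster spawners, with hidden-in-game markers, up to a set count and outside BP_NoSpawnLocation radii.
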(fn ConstructionScript
  (bind _minpoint (Variables|Default|GetMinPoint))
  (bind _maxpoint (Variables|Default|GetMaxPoint))
  (bind _meshlist (Variables|Default|GetMeshList))
  (bind _minscale (Variables|Default|GetMinScale))
  (bind _maxscale (Variables|Default|GetMaxScale))
  (bind _returnvalue (Math|Random|RandomFloatinRange _minscale _maxscale))
  (bind (_x _y) (Math|Vector|BreakVector _minpoint))
  (bind (_x_2 _y_2) (Math|Vector|BreakVector _maxpoint))
  (bind _returnvalue_2 (Math|Random|RandomFloatinRange _x _x_2))
  (bind _returnvalue_3 (Math|Random|RandomFloatinRange _y _y_2))
  (bind _returnvalue_4 (* _returnvalue 3e+04))
  (bind _returnvalue_5 (Math|Vector|MakeVector _returnvalue_2 _returnvalue_3 1e+05))
  ;[1 1 1] While There Are More Trees To Spawn
  (while (< (LocalVariables|GetLocalTreeCount) (Variables|Default|GetNumberOfTreesToSpawn))
    ;[1 1 1] Find Object Directly Beneath
    (Actor|GetAllActorsOfClass "/Script/Engine.Volume")
    (bind _outhit (Collision|LineTraceByChannel _returnvalue_5 (- _returnvalue_5 "0, 0,200000.000000") "TraceTypeQuery1" false 0 "None"))
    ;[1 1 1] If It Is Landscape
    (Utilities|Casting|CastToLandscape (.HitActor (Collision|BreakHitResult _outhit)))
    (bind _output_get (LocalVariables|SetLocalLocation (.Location (Collision|BreakHitResult _outhit))))
    ;[1 1 1] Don't Put On Steep Landscape
    (if (> (.Z (Math|Vector|BreakVector (.ImpactNormal (Collision|BreakHitResult _outhit)))) 0.65)
      ;[1 1 1] Stay Above Sea Level
      (if (>= (.Z (Math|Vector|BreakVector _output_get)) (Variables|Default|GetMinimumElevation))
        ;[1 1 1] Not Too Close To Existing Trees
        (bind _array_element (Utilities|Array|ForEachLoopwithBreak (Actor|GetComponentsByClass "/Script/Engine.StaticMeshComponent") :!label _label)
          (:LoopBody
            (Utilities|IsValid _array_element
              (:Is%20Valid
                (if (< (Math|Vector|VectorLengthSquared (- (Transformation|GetWorldLocation _array_element) (LocalVariables|GetLocalLocation))) (Variables|Default|GetMinimumDistanceBetweenTreesSquared))
                  (Variables|Default|SetStopNow true)
                  (goto _label Break)))))
          (:Completed
            (if (Variables|Default|GetStopNow)
              (Variables|Default|SetStopNow false)
              (else
                ;[1 1 1] Spawn Tree
                (bind _returnvalue_6 (AddComponent|AddStaticMeshComponent false (Math|Transform|MakeTransform (LocalVariables|GetLocalLocation) (Class|KismetMathLibrary|MakeRot 0.0 (Math|Random|RandomFloatinRange 0.0 3.6e+02) 0.0) (Math|Conversions|ToVector(Float) (Math|Random|RandomFloatinRange (Variables|Default|GetMinScale) (Variables|Default|GetMaxScale))))))
                (Components|StaticMesh|SetStaticMesh _returnvalue_6 (Utilities|Array|Get(acopy) _meshlist (Math|Random|RandomInteger (Utilities|Array|Length _meshlist))))
                (Collision|SetCollisionResponsetoAllChannels _returnvalue_6 "ECR_Block")
                (Rendering|SetCastShadow _returnvalue_6 true)
                (Collision|SetCollisionResponsetoChannel _returnvalue_6 "ECC_Camera" "ECR_Ignore")
                (Transformation|SetWorldLocation _returnvalue_6 (LocalVariables|GetLocalLocation) false)
                ;[1 1 1] Spawn Repel Sphere At Top Of Tree
                (bind _returnvalue_7 (AddComponent|AddBPRepellingSphere))
                (Utilities|IsValid _returnvalue_7
                  (:Is%20Valid
                    (Variables|/Game/Speedtree/BP_RepellingSphere.BP_RepellingSphere_C|SetTreePlacer _returnvalue_7 self)
                    (bind _output_get_2 (Variables|/Game/Speedtree/BP_RepellingSphere.BP_RepellingSphere_C|SetCenterPoint _returnvalue_7 (+ (LocalVariables|GetLocalLocation) (Math|Vector|MakeVector 0.0 0.0 _returnvalue_4))))
                    (bind _output_get_3 (Variables|/Game/Speedtree/BP_RepellingSphere.BP_RepellingSphere_C|SetRadius _returnvalue_7 _returnvalue_4))
                    ;[1 1 1] Show Collision Sphere If Requested
                    (if (Variables|Default|GetShowRepelSpheres)
                      (bind _returnvalue_8 (AddComponent|AddStaticMeshComponent false (Math|Conversions|ToTransform(Vector) _output_get_2)))
                      (Utilities|IsValid _returnvalue_8
                        (:Is%20Valid
                          (Components|StaticMesh|SetStaticMesh _returnvalue_8 "/Game/Speedtree/Shape_Sphere.Shape_Sphere")
                          (Transformation|SetWorldScale3D _returnvalue_8 (* "0.010000,0.010000,0.010000" _output_get_3))
                          (Transformation|SetWorldLocation _returnvalue_8 _output_get_2 false))))
                    ;[1 1 1] Remove One From Trees Spawned
                    (LocalVariables|SetLocalTreeCount (+ (LocalVariables|GetLocalTreeCount) 1))
                    (if (< (LocalVariables|GetLocalSpawnerCount) (Variables|Default|GetNumberOfEnemySpawnersToSpawn))
                      ;[1 1 1] Check If Location Is Near A Forbidden Spawning Area
                      (bind _outactors (Actor|GetAllActorsOfClass "/Game/Speedtree/BP_NoSpawnLocation.BP_NoSpawnLocation_C"))
                      (bind _array_element_2 (Utilities|Array|ForEachLoopwithBreak _outactors :!label _label_2)
                        (:LoopBody
                          (Utilities|IsValid _array_element_2
                            (:Is%20Valid
                              (if (<= (Math|Vector|VectorLength (- (Transformation|GetWorldLocation (Variables|/Game/Speedtree/BP_NoSpawnLocation.BP_NoSpawnLocation_C|GetSphere _array_element_2)) (LocalVariables|GetLocalLocation))) (Variables|/Game/Speedtree/BP_NoSpawnLocation.BP_NoSpawnLocation_C|GetRadius _array_element_2))
                                (Variables|Default|SetStopNow true)
                                (goto _label_2 Break)))))
                        (:Completed
                          (if (Variables|Default|GetStopNow)
                            (Variables|Default|SetStopNow false)
                            (else
                              ;[1 1 1] Add Spawner Component
                              (bind _returnvalue_9 (AddComponent|AddBPMonsterSpawnerComponent false (Math|Transform|MakeTransform (LocalVariables|GetLocalLocation))))
                              (Utilities|IsValid _returnvalue_9
                                (:Is%20Valid
                                  (Variables|/Game/Blueprints/Monsters/BP_MonsterSpawnerComponent.BP_MonsterSpawnerComponent_C|SetLocation _returnvalue_9 (+ (LocalVariables|GetLocalLocation) "0, 0,150.000000"))
                                  (bind _returnvalue_10 (AddComponent|AddStaticMeshComponent false (Math|Transform|MakeTransform (LocalVariables|GetLocalLocation))))
                                  (Utilities|IsValid _returnvalue_10
                                    (:Is%20Valid
                                      (Components|StaticMesh|SetStaticMesh _returnvalue_10 "/Game/Models/Attacks/slimeballpink.slimeballpink")
                                      (Transformation|SetWorldLocation _returnvalue_10 (+ (LocalVariables|GetLocalLocation) "0.000000,0.000000,250.000000") false)
                                      (Transformation|SetWorldScale3D _returnvalue_10 "20.000000,20.000000,20.000000")
                                      (Rendering|SetVisibility _returnvalue_10 true false)
                                      (Development|SetHiddeninGame _returnvalue_10 true false)
                                      (Collision|SetCollisionEnabled _returnvalue_10 "NoCollision")
                                      ;[1 1 1] Lower Spawner Count By One
                                      (LocalVariables|SetLocalSpawnerCount (+ (LocalVariables|GetLocalSpawnerCount) 1)))))))))))))))))))))