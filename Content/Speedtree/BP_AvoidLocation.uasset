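; BP_AvoidLocation is a Speedtree-folder actor or component with an editable size, likely marking an area to avoid.
; Its construction script folds Multiply into Scale and resets Multiply to 1, so the multiplier acts as a one-shot resize.
; It then sets world scale to Scale divided by 100, converting units to scale.
; Both branches of the IsSpherical check apply the identical scale.
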(fn `UserConstructionScript`
  (bind _returnvalue (/ (`self.Scale`) 100.0))
  (set `self.Scale` (* (`self.Scale`) (`self.Multiply`)))
  (set `self.Multiply` 1.0)
  (if (`self.IsSpherical`)
    (`SceneComponent.SetWorldScale3D` _returnvalue)
    (else
      (`SceneComponent.SetWorldScale3D` _returnvalue))))