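; Repelling sphere for the Speedtree setup that pushes characters outward from a center point.
; Each tick it checks the TreePlacer's character list for walking or falling characters within a squared radius cached at initialization.
; It skips any with Landscape as the hit of a short downward trace.
; The rest get a delta-time-scaled force, lerped center to edge by squared distance, then have their velocity capped.
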(event `self.ReceiveInitializeComponent`
  (bind _radius (`self.Radius`))
  ;[1 1 1] Set Radius Squared Once
  (set `self.RadiusSquared` (* _radius _radius)))

(event `self.ReceiveTick`
  (params (DeltaSeconds :type "Float (single-precision)"))
  ;[1 1 1] Only Apply To Character Actors
  (for _array_element (`/Game/Speedtree/BP_TreePlacer.Characters` (`self.TreePlacer`))
    ;[1 1 1] Do Not Apply Force If Actor Is Close To Ground
    (if (and (<= (`KismetMathLibrary.VSizeSquared` (- (`Actor.K2_GetActorLocation` _array_element) (`self.CenterPoint`))) (`self.RadiusSquared`)) (or (`NavMovementComponent.IsFalling` _array_element) (`CharacterMovementComponent.IsWalking` _array_element)))
      (bind _returnvalue (`Actor.K2_GetActorLocation` _array_element))
      (bind _outhit (`KismetSystemLibrary.LineTraceSingle` _returnvalue (- _returnvalue (0.0 0.0 500.0)) "TraceTypeQuery1"))
      (cast `Landscape` (`.HitActor` (`GameplayStatics.BreakHitResult` _outhit))
        (:`CastFailed`
          (bind _charactermovement (`Character.CharacterMovement` _array_element))
          (bind _returnvalue_2 (`Actor.K2_GetActorLocation` _array_element))
          (`CharacterMovementComponent.AddForce` _charactermovement (* (`KismetMathLibrary.GetDirectionVector` (`self.CenterPoint`) _returnvalue_2) (* (`GameplayStatics.GetWorldDeltaSeconds`) (`KismetMathLibrary.Lerp` (`self.ForceAtCenter`) (`self.ForceAtEdge`) (/ (`KismetMathLibrary.VSizeSquared` (- _returnvalue_2 (`self.CenterPoint`))) (`self.RadiusSquared`))))))
          (bind _velocity (`MovementComponent.Velocity` _charactermovement))
          (if (> (`KismetMathLibrary.VSize` _velocity) (`self.LimitForceMagnitude`))
            (set `MovementComponent.Velocity` (* (`KismetMathLibrary.Normal` _velocity) (`self.LimitForceMagnitude`)) _charactermovement)))))))