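; BP_EnvironmentDamage is a hazard volume that damages the player's DragonCharacter over time while inside its DamageBox.
; Begin and end overlaps with any DragonCharacter toggle the IsDamaging flag.
; While the flag is set, Tick drains Health, Stamina and Breath by per-second amounts scaled by DeltaSeconds.
; The drain always targets player character 0, whichever dragon triggered the overlap.
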(event `self.DamageBox.OnComponentBeginOverlap`
  (params (OtherActor :type "Actor Object Reference") (OtherComp :type "PrimitiveComponent Object Reference") (OtherBodyIndex :type Integer) (bFromSweep :type Boolean) (SweepResult :type "EngineTypes.HitResult Structure (by ref)"))
  ;[1 1 1] Set as inside or outside of box
  (cast `/Game/Blueprints/DragonCharacter` OtherActor)
  (set `self.IsDamaging` true))

(event `self.DamageBox.OnComponentEndOverlap`
  (params (OtherActor :type "Actor Object Reference") (OtherComp :type "PrimitiveComponent Object Reference") (OtherBodyIndex :type Integer))
  ;[1 1 1] Set as inside or outside of box
  (cast `/Game/Blueprints/DragonCharacter` OtherActor)
  (set `self.IsDamaging` false))

(event `self.ReceiveTick`
  (params (DeltaSeconds :type "Float (single-precision)"))
  ;[1 1 1] Damage over time
  (if (`self.IsDamaging`)
    (bind _asdragon_character (cast `/Game/Blueprints/DragonCharacter` (`GameplayStatics.GetPlayerCharacter` 0)))
    (set `/Game/Blueprints/DragonCharacter.Health` (- (`/Game/Blueprints/DragonCharacter.Health` _asdragon_character) (* (`self.HealthDamageAmount`) DeltaSeconds)) _asdragon_character)
    (set `/Game/Blueprints/DragonCharacter.Stamina` (- (`/Game/Blueprints/DragonCharacter.Stamina` _asdragon_character) (* (`self.StaminaDamageAmount`) DeltaSeconds)) _asdragon_character)
    (set `/Game/Blueprints/DragonCharacter.Breath` (- (`/Game/Blueprints/DragonCharacter.Breath` _asdragon_character) (* (`self.BreathDamageAmount`) DeltaSeconds)) _asdragon_character)))

(fn `UserConstructionScript`)