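; Trace helper functions that find what lies beneath an actor and fit it to the landscape.
; Each casts a long downward line trace against WorldStatic objects: FindObjectBeneath returns the first hit, while the others filter multi-hits for Landscape.
; PlaceAgainstGround moves the actor to the hit, deriving pitch and roll from the surface normal and yaw from Character.
; FindLocationOnGround returns the landscape point or falls back to the actor's location; its Hit output is never set.
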(fn FindObjectBeneath
  (params (Actor :type Actor%20Object%20Reference))
  (bind _returnvalue (Transformation|GetActorLocation Actor))
  (bind (_outhit _returnvalue_2) (Collision|LineTraceForObjects 0 _returnvalue (- _returnvalue "0, 0,100000.000000") (Utilities|Array|MakeArray "ObjectTypeQuery1") false 0 "None"))
  (return _returnvalue_2 (.HitActor (Collision|BreakHitResult _outhit)) (.HitComponent (Collision|BreakHitResult _outhit))))

(fn PlaceAgainstGround
  (params (Character :type Character%20Object%20Reference) (Actor :type Actor%20Object%20Reference))
  (bind _returnvalue (Transformation|GetActorLocation Actor))
  (bind _returnvalue_2 (Transformation|GetWorldRotation Character))
  (bind (_outhits _returnvalue_3) (Class|KismetSystemLibrary|LineTraceMultiforObjects 0 _returnvalue (- _returnvalue "0, 0,100000.000000") (Utilities|Array|MakeArray "ObjectTypeQuery1") false 0 "None" true))
  (for _array_element _outhits
    (Utilities|Casting|CastToLandscape 0)
    (if _returnvalue_3
      (Transformation|SetActorRotation Actor (Math|Interpolation|RInterpTo _returnvalue_2 (Class|KismetMathLibrary|MakeRot (.Pitch (Class|KismetMathLibrary|BreakRot (Class|KismetMathLibrary|MakeRotfromYZ (Math|Vector|GetRightVector Character) (.ImpactNormal (Collision|BreakHitResult _array_element))))) (.Yaw (Class|KismetMathLibrary|BreakRot _returnvalue_2)) (.Roll (Class|KismetMathLibrary|BreakRot (Math|Rotator|MakeRotfromXZ (Math|Vector|GetForwardVector Character) (.ImpactNormal (Collision|BreakHitResult _array_element)))))) (Utilities|Time|GetWorldDeltaSeconds) 0.0))
      (Transformation|SetActorLocation Actor (.Location (Collision|BreakHitResult _array_element)) false))))

(fn FindLocationonGround
  (params (Actor :type Actor%20Object%20Reference))
  (bind _returnvalue (Transformation|GetActorLocation Actor))
  ;[1 1 1] Get Array Of Static Actors Beneath The Actor
  (bind _outhits (Class|KismetSystemLibrary|LineTraceMultiforObjects 0 _returnvalue (- _returnvalue "0, 0,100000.000000") (Utilities|Array|MakeArray "ObjectTypeQuery1") false 0 "None" true))
  ;[1 1 1] For Each Actor In Array
  (for _array_element _outhits
    ;[1 1 1] If Finds A Landscape, Set That As The Location
    (Utilities|Casting|CastToLandscape (.HitActor (Collision|BreakHitResult _array_element)))
    (LocalVariables|SetLocalLocation (.Location (Collision|BreakHitResult _array_element))))
  ;[1 1 1] If Location Wasn't Set By Loop, Set It To Actor's Own Location Instead
  (if (Math|Vector|NotEqual(Vector) (LocalVariables|GetLocalLocation) "0, 0, 0" 0.0)
    _
    (else
      (LocalVariables|SetLocalLocation _returnvalue)))
  ;[1 1 1] Return
  (return (LocalVariables|GetLocalHit) (LocalVariables|GetLocalLocation)))