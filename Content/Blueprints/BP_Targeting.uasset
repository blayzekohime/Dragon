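; BP_Targeting is a lock-on component that lets the dragon player find, mark and cycle through enemy characters and destructibles.
; Toggling lock runs successively larger box traces forward from the dragon's DropLocation to fill EnemiesInSight, then shows the selected target's arrow.
; Cycling and kill removal update the index and arrows, while GetLockedEnemy returns the target's location and flags destructibles as castle.
; Tick scales AI target arrows by distance to the player.
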(event `self.ReceiveTick`
  (params (DeltaSeconds :type "Float (single-precision)"))
  (bind _hastargets (`self.GetHasTargets`))
  (if _hastargets
    (bind _asaicharacter (cast `/Game/Blueprints/AI/AICharacter` (`KismetArrayLibrary.Array_Get` (`self.EnemiesInSight`) (`self.LockedTargetIndex`))))
    (bind _targetarrow (`/Game/Blueprints/AI/AICharacter.TargetArrow` _asaicharacter))
    (bind _returnvalue (/ (`Actor.GetDistanceTo` _asaicharacter (`GameplayStatics.GetPlayerCharacter` 0)) 1000.0))
    (`SceneComponent.SetWorldScale3D` _targetarrow (`KismetMathLibrary.MakeVector` _returnvalue _returnvalue (.z (`SceneComponent.K2_GetComponentScale` _targetarrow))))))

(event `self.ReceiveInitializeComponent`)

(fn `CycleThroughTargets`
  (bind _enemiesinsight (`self.EnemiesInSight`))
  (bind _enemiesinsight_2 (`self.EnemiesInSight`))
  (bind _lockedtargetindex (`self.LockedTargetIndex`))
  (bind _enemiesinsight_3 (`self.EnemiesInSight`))
  (bind _item (`KismetArrayLibrary.Array_Get` _enemiesinsight_2))
  (bind _item_2 (`KismetArrayLibrary.Array_Get` _enemiesinsight _lockedtargetindex))
  (bind _returnvalue (+ _lockedtargetindex 1))
  (bind _item_3 (`KismetArrayLibrary.Array_Get` _enemiesinsight_2 (`KismetArrayLibrary.Array_LastIndex` _enemiesinsight_2)))
  ;[1 1 1] Check to See if we still Have Targets
  (if (== (`KismetArrayLibrary.Array_Length` (`self.EnemiesInSight`)) 0)
    (set `self.TotalEnemiesInSight` 0)
    (set `self.HasTargets` false)
    (set `self.LockIsOn` false)
    (elif (> _returnvalue (`KismetArrayLibrary.Array_LastIndex` _enemiesinsight))
      (bind _output_get (set `self.LockedTargetIndex` 0))
      ;[1 1 1] If we are going back to Index 0
      ;;[1 1 1] If there is only One Target
      (if (> (`KismetArrayLibrary.Array_Length` _enemiesinsight_3) 1)
        (bind _asaicharacter (cast `/Game/Blueprints/AI/AICharacter` _item_3)
          (:`then`
            _)
          (:`CastFailed`
            (bind _asbp_destructible (cast `/Game/Blueprints/AI/Castle/BP_Destructible` _item_3))))
        (bind _asaicharacter_2 (cast `/Game/Blueprints/AI/AICharacter` _item)
          (:`then`
            _)
          (:`CastFailed`
            (bind _asbp_destructible_2 (cast `/Game/Blueprints/AI/Castle/BP_Destructible` _item))))
        (`SceneComponent.SetHiddenInGame` (`/Game/Blueprints/AI/AICharacter.TargetArrow` _asaicharacter_2) false false)
        (`SceneComponent.SetHiddenInGame` (`/Game/Blueprints/AI/Castle/BP_Destructible.TargetArrow` _asbp_destructible_2) false false)
        (`SceneComponent.SetHiddenInGame` (`/Game/Blueprints/AI/AICharacter.TargetArrow` _asaicharacter) true false)
        (`SceneComponent.SetHiddenInGame` (`/Game/Blueprints/AI/Castle/BP_Destructible.TargetArrow` _asbp_destructible) true false)
        (else
          (bind _asaicharacter_3 (cast `/Game/Blueprints/AI/AICharacter` (`KismetArrayLibrary.Array_Get` _enemiesinsight_3 _output_get)))
          (`SceneComponent.SetHiddenInGame` (`/Game/Blueprints/AI/AICharacter.TargetArrow` _asaicharacter_3) false false)))
      (else
        (bind _asaicharacter_4 (cast `/Game/Blueprints/AI/AICharacter` _item_2)
          (:`then`
            ;[1 1 1] If we are just incrementing to next Index
            (`SceneComponent.SetHiddenInGame` (`/Game/Blueprints/AI/AICharacter.TargetArrow` _asaicharacter_4) true false)
            (`SceneComponent.SetHiddenInGame` (`/Game/Blueprints/AI/Castle/BP_Destructible.TargetArrow` (stale _asbp_destructible_4)) true false)
            (bind _output_get_2 (set `self.LockedTargetIndex` _returnvalue))
            (bind _item_4 (`KismetArrayLibrary.Array_Get` _enemiesinsight _output_get_2))
            (bind _asaicharacter_5 (cast `/Game/Blueprints/AI/AICharacter` _item_4)
              (:`then`
                _)
              (:`CastFailed`
                (bind _asbp_destructible_3 (cast `/Game/Blueprints/AI/Castle/BP_Destructible` _item_4))))
            (`SceneComponent.SetHiddenInGame` (`/Game/Blueprints/AI/AICharacter.TargetArrow` _asaicharacter_5) false false)
            (`SceneComponent.SetHiddenInGame` (`/Game/Blueprints/AI/Castle/BP_Destructible.TargetArrow` _asbp_destructible_3) false false))
          (:`CastFailed`
            (bind _asbp_destructible_4 (cast `/Game/Blueprints/AI/Castle/BP_Destructible` _item_2))))))))

(fn `GetHasTargets`
  (returns (HasTargets :type Boolean))
  ;[1 1 1] Do We Have Targets?
  (return (`self.HasTargets`)))

(fn `GetLockedEnemy`
  (returns (LockedEnemyNotFlying :type "Object.Vector Structure") (LockedEnemyFlying :type "Object.Vector Structure") (LockedWallNotFlying :type "Object.Vector Structure") (LockedWallFlying :type "Object.Vector Structure"))
  (bind _item (`KismetArrayLibrary.Array_Get` (`self.EnemiesInSight`) (`self.LockedTargetIndex`)))
  ;[1 1 1] Return the Vector location of Targeted Enemy
  (`/Engine/EditorBlueprintResources/StandardMacros.IsValid` _item
    (:`Is Valid`
      (bind _asdragon_character (cast `/Game/Blueprints/DragonCharacter` (`GameplayStatics.GetPlayerCharacter` 0)))
      ;[1 1 1] If the player is on the ground
      (bind _asaicharacter (cast `/Game/Blueprints/AI/AICharacter` _item)
        (:`then`
          (set `self.IsCastle` false))
        (:`CastFailed`
          (bind _asbp_destructible (cast `/Game/Blueprints/AI/Castle/BP_Destructible` _item))
          (set `self.IsCastle` true)))
      (bind _returnvalue (`SceneComponent.K2_GetComponentLocation` (`/Game/Blueprints/AI/AICharacter.LockingArrow` _asaicharacter)))
      (bind _returnvalue_2 (`SceneComponent.K2_GetComponentLocation` _asbp_destructible))
      (return _returnvalue _returnvalue _returnvalue_2 _returnvalue_2))))

(fn `GetPlayerLocation`
  (returns (NewParam :type "Object.Vector Structure"))
  (return (`SceneComponent.K2_GetComponentLocation` (`GameplayStatics.GetPlayerCharacter` 0))))

(fn `GetTargets`
  (bind _returnvalue (`KismetArrayLibrary.Array_Length` (`self.EnemiesInSight`)))
  (for _index (range 1 (+ (`self.NumberOfTraces`) 1))
    (bind _asdragon_character (cast `/Game/Blueprints/DragonCharacter` (`GameplayStatics.GetPlayerCharacter` 0)))
    (bind _outactors (`GameplayStatics.GetAllActorsOfClass` "/Game/Blueprints/BP_RangedAttack.BP_RangedAttack_C"))
    (bind _droplocation (`/Game/Blueprints/DragonCharacter.DropLocation` _asdragon_character))
    (bind _returnvalue_2 (`SceneComponent.GetForwardVector` _droplocation))
    (bind _returnvalue_3 (`KismetMathLibrary.Conv_IntToDouble` _index))
    (bind _returnvalue_4 (* (`self.StartHalfHeight`) _returnvalue_3))
    (bind _z (.z _returnvalue_4))
    (bind _returnvalue_5 (+ (`SceneComponent.K2_GetComponentLocation` _droplocation) (`KismetMathLibrary.MakeVector` (.x (* _returnvalue_2 (* (* _returnvalue_3 _z) 1.0))) (.y (* _returnvalue_2 (* (* _returnvalue_3 _z) 1.0))) (.z (* _returnvalue_2 (* (* _returnvalue_3 _z) 1.0))))))
    (bind (_outhit _returnvalue_6) (`KismetSystemLibrary.BoxTraceSingleForObjects` _returnvalue_5 (+ _returnvalue_5 (* _returnvalue_2 _z)) _returnvalue_4 (`SceneComponent.K2_GetComponentRotation` _droplocation) (`|MakeArray` "ObjectTypeQuery6" "ObjectTypeQuery3" :!type "EngineTypes.EObjectTypeQuery Enum") true _outactors "ForDuration"))
    ;[1 1 1] Add to Array if Visible
    (if _returnvalue_6
      (`KismetArrayLibrary.Array_Add` (`self.EnemiesInSight`) (`.HitActor` (`GameplayStatics.BreakHitResult` _outhit)))))
  ;[1 1 1] End of Loop Settings
  ;;[1 1 1] Has Targets
  (if (> _returnvalue 0)
    (set `self.TotalEnemiesInSight` _returnvalue)
    (set `self.HasTargets` true)
    (else
      ;;[1 1 1] No Targets
      (set `self.TotalEnemiesInSight` 0)
      (set `self.HasTargets` false))))

(fn `RemoveKilledTarget`
  (params (KilledTarget :type "Actor Object Reference"))
  (bind _asbp_destructible (cast `/Game/Blueprints/AI/Castle/BP_Destructible` KilledTarget)
    (:`then`
      (`SceneComponent.SetVisibility` (`/Game/Blueprints/AI/Castle/BP_Destructible.TargetArrow` _asbp_destructible) false false))
    (:`CastFailed`
      _))
  (bind _returnvalue (`KismetArrayLibrary.Array_RemoveItem` (`self.EnemiesInSight`) KilledTarget))
  (if _returnvalue
    (`self.CycleThroughTargets`)))

(fn `ToggleLocking`
  (bind _enemiesinsight (`self.EnemiesInSight`))
  (bind _item (`KismetArrayLibrary.Array_Get` _enemiesinsight (`self.LockedTargetIndex`)))
  (bind _output_get (set `self.LockIsOn` (not (`self.LockIsOn`))))
  (if _output_get
    ;[1 1 1] Lock Is On
    (`KismetArrayLibrary.Array_Clear` _enemiesinsight)
    (`self.GetTargets`)
    (if (`self.HasTargets`)
      (bind _asaicharacter (cast `/Game/Blueprints/AI/AICharacter` _item)
        (:`then`
          _)
        (:`CastFailed`
          (bind _asbp_destructible (cast `/Game/Blueprints/AI/Castle/BP_Destructible` _item))
          (bind _targetarrow (`/Game/Blueprints/AI/Castle/BP_Destructible.TargetArrow` _asbp_destructible))
          (`SceneComponent.K2_SetWorldLocation` _targetarrow (+ (`SceneComponent.K2_GetComponentLocation` _targetarrow) (0.0 0.0 3500.0)) false)))
      (`SceneComponent.SetHiddenInGame` (`/Game/Blueprints/AI/AICharacter.TargetArrow` _asaicharacter) false false)
      (`SceneComponent.SetHiddenInGame` _targetarrow false false))
    (else
      ;[1 1 1] Lock Is Off
      (if (`self.HasTargets`)
        (bind _asaicharacter_2 (cast `/Game/Blueprints/AI/AICharacter` _item)
          (:`then`
            _)
          (:`CastFailed`
            (bind _asbp_destructible_2 (cast `/Game/Blueprints/AI/Castle/BP_Destructible` _item))))
        (`SceneComponent.SetHiddenInGame` (`/Game/Blueprints/AI/AICharacter.TargetArrow` _asaicharacter_2) true false)
        (`SceneComponent.SetHiddenInGame` (`/Game/Blueprints/AI/Castle/BP_Destructible.TargetArrow` _asbp_destructible_2) true false)
        (`KismetArrayLibrary.Array_Clear` _enemiesinsight)
        (set `self.HasTargets` false)
        (set `self.TotalEnemiesInSight` 0)))))