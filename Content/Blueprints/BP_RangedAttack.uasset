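; Configurable physics projectile for ranged attacks by the player's dragon or by enemies, exploding on hitting an opposing character.
; Init sets visuals, damage and lifespan, then launches player shots at the targeting component's locked enemy or castle wall, else forward; enemy shots follow a supplied vector.
; Explode damages AI characters within the radius sphere, or the player by distance check.
; Tick zeroes angular velocity to prevent spinning, and mesh hits destroy the actor.
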(event `self.ReceiveBeginPlay`)

(event `Explode`
  (bind _returnvalue (`GameplayStatics.GetPlayerCharacter` 0))
  ;[1 1 1] Spawn Explosion
  (`GameplayStatics.SpawnEmitterAtLocation` (`ParticleSystemComponent.Template` (`self.ParticlesExplosion`)) (`self.K2_GetActorLocation`))
  ;[1 1 1] Is It The Player's?
  (if (`self.IsPlayers`)
    ;[1 1 1] It's a Player's Projectile
    (for _array_element (`PrimitiveComponent.GetOverlappingActors` (`self.ExplosionRadius`) "/Game/Blueprints/AI/AICharacter.AICharacter_C")
      (bind _asaicharacter (cast `/Game/Blueprints/AI/AICharacter` _array_element))
      (`/Engine/EditorBlueprintResources/StandardMacros.IsValid` _asaicharacter
        (:`Is Valid`
          ;[1 1 1] Damage Enemies In Range
          (`/Game/Blueprints/AI/AICharacter.Hurt` _asaicharacter (`self.DamageHealth`) (`self.DamageStamina`) (`self.DamageBreath`) (`GameplayStatics.GetPlayerCharacter` 0))
          (`KismetSystemLibrary.Delay` 0.5 :!label _label)
          (`self.K2_DestroyActor`))))
    (goto _label)
    (else
      ;[1 1 1] It's The Enemy's Projectile
      (if (<= (`self.GetDistanceTo` _returnvalue) (`SphereComponent.SphereRadius` (`self.ExplosionRadius`)))
        (bind _asdragon_character (cast `/Game/Blueprints/DragonCharacter` _returnvalue))
        (`/Game/Blueprints/DragonCharacter.Hurt` _asdragon_character (`self.DamageHealth`) (`self.DamageStamina`) (`self.DamageBreath`))
        (goto _label)))))

(event `self.StaticMesh.OnComponentHit`
  (params (OtherActor :type "Actor Object Reference") (OtherComp :type "PrimitiveComponent Object Reference") (NormalImpulse :type "Object.Vector Structure") (Hit :type "EngineTypes.HitResult Structure (by ref)"))
  (`self.K2_DestroyActor`))

(event `self.ReceiveTick`
  (params (DeltaSeconds :type "Float (single-precision)"))
  ;[1 1 1] Keep Straight Projectiles From SPinning In Flight
  (`PrimitiveComponent.SetPhysicsAngularVelocity` (`self.ProjectileMovement`) (0.0 0.0 0.0) false "None"))

(event `self.ReceiveHit`
  (params (MyComp :type "PrimitiveComponent Object Reference") (Other :type "Actor Object Reference") (OtherComp :type "PrimitiveComponent Object Reference") (bSelfMoved :type Boolean) (HitLocation :type "Object.Vector Structure") (HitNormal :type "Object.Vector Structure") (NormalImpulse :type "Object.Vector Structure") (Hit :type "EngineTypes.HitResult Structure (by ref)"))
  (if (`self.IsPlayers`)
    (cast `/Game/Blueprints/AI/AICharacter` Other)
    (else
      (cast `/Game/Blueprints/DragonCharacter` Other)))
  (`self.Explode`))

(fn `GetIsPlayers`
  (returns (IsPlayers :type Boolean))
  (return (`self.IsPlayers`)))

(fn `Init`
  (params (StaticMesh :type "StaticMesh Object Reference") (ParticlesBase :type "ParticleSystem Object Reference") (ParticlesExplosion :type "ParticleSystem Object Reference") (ExplosionRadius :type "Float (double-precision)" :default 0.0) (Force :type "Float (double-precision)" :default 0.0) (LifeSpan :type "Float (double-precision)" :default 0.0) (DamageHealth :type "Float (double-precision)") (DamageStamina :type "Float (double-precision)" :default 0.0) (DamageBreath :type "Float (double-precision)" :default 0.0) (UseGravity :type Boolean :default false) (IsPlayers :type Boolean :default false) (IsVisible :type Boolean :default false) (Variance :type "Object.Vector Structure" :default (0.0 0.0 0.0)))
  (bind _returnvalue (`SceneComponent.K2_GetComponentLocation`))
  (bind _returnvalue_2 (`SceneComponent.K2_GetComponentLocation`))
  (bind _returnvalue_3 (`self.GetActorForwardVector` (`GameplayStatics.GetPlayerCharacter` 0)))
  (bind _returnvalue_4 (`SceneComponent.K2_GetComponentLocation` (`self.StaticMesh`)))
  (`StaticMeshComponent.SetStaticMesh` StaticMesh)
  (`ParticleSystemComponent.SetTemplate` (`self.ParticlesBase`) ParticlesBase)
  (`ParticleSystemComponent.SetTemplate` (`self.ParticlesExplosion`) ParticlesExplosion)
  (`SphereComponent.SetSphereRadius` ExplosionRadius)
  (if IsPlayers
    (bind _asdragon_character (cast `/Game/Blueprints/DragonCharacter` (`GameplayStatics.GetPlayerCharacter` 0)))
    (`/Engine/EditorBlueprintResources/StandardMacros.IsValid` _asdragon_character
      (:`Is Valid`
        (bind _bp_targeting (`/Game/Blueprints/DragonCharacter.BP_Targeting` _asdragon_character))
        ;[1 1 1] Player Shoot Fireball in Direction of Locked Enemy
        (bind _hastargets (`/Game/Blueprints/BP_Targeting.GetHasTargets` _bp_targeting))
        (if _hastargets
          (bind (_lockedenemynotflying _lockedenemyflying _lockedwallnotflying) (`/Game/Blueprints/BP_Targeting.GetLockedEnemy` _bp_targeting))
          (if (`/Game/Blueprints/DragonCharacter.IsFlying` _asdragon_character)
            (bind _iscastle (`/Game/Blueprints/BP_Targeting.IsCastle` _bp_targeting))
            (if _iscastle
              (bind _returnvalue_5 (`KismetMathLibrary.GetDirectionVector` _returnvalue_2 _lockedwallnotflying))
              ;;[1 1 1] If the player is flying
              (`PrimitiveComponent.AddForceAtLocation` (* _returnvalue_5 Force) _returnvalue_4)
              (`PrimitiveComponent.AddImpulseAtLocation` (* _returnvalue_5 100000.0) _returnvalue_4)
              (else
                (bind _returnvalue_6 (`KismetMathLibrary.GetDirectionVector` _returnvalue_2 _lockedenemynotflying))
                (`PrimitiveComponent.AddForceAtLocation` (* _returnvalue_6 Force) _returnvalue_4)
                (`PrimitiveComponent.AddImpulseAtLocation` (* _returnvalue_6 100000.0) _returnvalue_4)))
            (elif _iscastle
              (bind _returnvalue_7 (`KismetMathLibrary.GetDirectionVector` _returnvalue _lockedwallnotflying))
              (`PrimitiveComponent.AddForceAtLocation` (* _returnvalue_7 Force) _returnvalue_4)
              (`PrimitiveComponent.AddImpulseAtLocation` (* _returnvalue_7 100000.0) _returnvalue_4)
              (else
                (bind _returnvalue_8 (`KismetMathLibrary.GetDirectionVector` _returnvalue _lockedenemynotflying))
                (`PrimitiveComponent.AddForceAtLocation` (* _returnvalue_8 Force) _returnvalue_4)
                (`PrimitiveComponent.AddImpulseAtLocation` (* _returnvalue_8 100000.0) _returnvalue_4))))
          (else
            ;[1 1 1] Player Shoot Fireball Forward
            (`PrimitiveComponent.AddForceAtLocation` (* _returnvalue_3 Force) _returnvalue_4)
            (`PrimitiveComponent.AddImpulseAtLocation` (* _returnvalue_3 100000.0) _returnvalue_4)))))
    (else
      ;[1 1 1] Enemy is firing, Shoot in direction the AI provided
      (`PrimitiveComponent.AddImpulseAtLocation` (* Variance Force) _returnvalue_4)))
  (`self.SetLifeSpan` LifeSpan)
  (set `self.DamageHealth` DamageHealth)
  (set `self.DamageStamina` DamageStamina)
  (set `self.DamageBreath` DamageBreath)
  (`PrimitiveComponent.SetEnableGravity` (`self.StaticMesh`) UseGravity)
  (set `self.IsPlayers` IsPlayers)
  (`SceneComponent.SetVisibility` (`self.StaticMesh`) IsVisible false))

(fn `UserConstructionScript`)