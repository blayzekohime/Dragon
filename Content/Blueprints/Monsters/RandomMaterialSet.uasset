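; RandomMaterialSet is a Blueprint in the Monsters folder that holds a set of materials and hands out random or indexed picks.
; AddMaterial and ClearMaterials maintain the Materials array, with additions kept unique.
; GetRandomMaterial and GetMaterial each return a material and a success flag, using None on failure.
; GetMaterial's bounds check is inverted, passing only when Index exceeds the array length, so valid indices fail.
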(event EventBeginPlay)

(event EventActorBeginOverlap
  (params (OtherActor :type Actor%20Object%20Reference)))

(event EventTick
  (params (DeltaSeconds :type Float%20%28single-precision%29)))

(fn ConstructionScript)

(fn GetRandomMaterial
  (bind _materials (Variables|Default|GetMaterials))
  (bind _returnvalue (Utilities|Array|Length _materials))
  (bind _returnvalue_2 (> _returnvalue 0))
  ;[1 1 1] Check If Array Has Any Members
  (if _returnvalue_2
    ;[1 1 1] Return A Random Material From The Array
    (LocalVariables|SetReturnedMaterial (Utilities|Array|Get(acopy) _materials (Math|Random|RandomInteger _returnvalue)))
    (else
      ;[1 1 1] Return A Null Material
      (LocalVariables|SetReturnedMaterial 0)))
  (return (LocalVariables|GetReturnedMaterial) _returnvalue_2))

(fn GetMaterial
  (params (Index :type Integer))
  (bind _materials (Variables|Default|GetMaterials))
  (bind _returnvalue (Utilities|Array|Length _materials))
  (bind _returnvalue_2 (> _returnvalue 0))
  (bind _returnvalue_3 (< _returnvalue Index))
  (bind _returnvalue_4 (and _returnvalue_2 _returnvalue_3))
  ;[1 1 1] Check If Index Between Zero and Length
  (if _returnvalue_4
    ;[1 1 1] Return Material At Index
    (LocalVariables|SetReturnedMaterial (Utilities|Array|Get(acopy) (Variables|Default|GetMaterials) Index))
    (else
      ;[1 1 1] Return Null Material
      (LocalVariables|SetReturnedMaterial 0)))
  (return (LocalVariables|GetReturnedMaterial) _returnvalue_4))

(fn AddMaterial
  (params (Material :type Material%20Object%20Reference))
  (bind _returnvalue (Utilities|Array|AddUnique (Variables|Default|GetMaterials) Material))
  (return _returnvalue))

(fn ClearMaterials
  (Utilities|Array|Clear (Variables|Default|GetMaterials)))