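; Monster spawner component that keeps one enemy, either a LimeJelly or a Whiplash AI character picked at random, alive at a stored location.
; While active, Tick counts up a timer whenever the spawned enemy is missing or dead, then destroys the old actor and spawns a replacement after a set delay.
; A player-proximity check that would gate spawning and despawn distant enemies is present but disconnected, so it never runs.
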(event `self.ReceiveTick`
  (params (DeltaSeconds :type "Float (single-precision)"))
  (bind _spawntimer (`self.SpawnTimer`))
  (bind _spawnedenemy (`self.SpawnedEnemy`))
  (bind _spawnedenemy_2 (`self.SpawnedEnemy`))
  (bind _returnvalue (`KismetMathLibrary.Conv_VectorToTransform` (`self.Location`)))
  (if (`self.Active`)
    ;[1 1 1] Spawn After Specific Number Of Seconds When The Spawned Enemy Dies
    (if (or (not (`KismetSystemLibrary.IsValid` _spawnedenemy)) (<= (`/Game/Blueprints/AI/AICharacter.Health` _spawnedenemy) 0.0))
      (if (> _spawntimer (`self.SecondsToNewSpawn`))
        (set `self.SpawnTimer` 0.0)
        ;[1 1 1] Destroy The Old One If It Exists
        (`/Engine/EditorBlueprintResources/StandardMacros.IsValid` _spawnedenemy_2
          (:`Is Valid`
            (`self.K2_DestroyActor` _spawnedenemy_2))
          (:`Is Not Valid`
            _))
        ;[0.09728 1 0.4109] Spawn It
        (if (`KismetMathLibrary.RandomBool`)
          (bind _returnvalue_2 (`|SpawnActorFromClass` "/Game/Blueprints/AI/Enemies/LimeJellyAICharacter.LimeJellyAICharacter_C" _returnvalue true))
          (set `self.SpawnedEnemy` _returnvalue_2)
          (else
            (bind _returnvalue_3 (`|SpawnActorFromClass` "/Game/Blueprints/AI/Enemies/WhiplashAICharacter.WhiplashAICharacter_C" _returnvalue true))
            (set `self.SpawnedEnemy` _returnvalue_3)))
        (else
          (set `self.SpawnTimer` (+ _spawntimer (`GameplayStatics.GetWorldDeltaSeconds`))))))))

(event `self.ReceiveInitializeComponent`)