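; BP_MonsterSpawner is a placed actor that respawns a single monster while the DragonCharacter is inside its sphere.
; On Tick, once its monster is missing or dead, a timer runs before it replaces it with a random LimeJelly or Whiplash AI character.
; Each spawn registers with BP_MonsterSpawnerControl, which caps the monster count.
; The construction script uses a vertical trace to position the spawner above the Landscape.
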(event `self.ReceiveBeginPlay`
  (bind _outactors (`GameplayStatics.GetAllActorsOfClass` "/Game/Blueprints/Monsters/BP_MonsterSpawnerControl.BP_MonsterSpawnerControl_C"))
  (set `self.Controller` (`KismetArrayLibrary.Array_Get` _outactors)))

(event `self.ReceiveTick`
  (params (DeltaSeconds :type "Float (single-precision)"))
  (bind _controller (`self.Controller`))
  (bind _spawnedenemy (`self.SpawnedEnemy`))
  (bind _spawntimer (`self.SpawnTimer`))
  (bind _spawnedenemy_2 (`self.SpawnedEnemy`))
  (bind _returnvalue (`KismetMathLibrary.Conv_VectorToTransform` (`self.K2_GetActorLocation`)))
  ;[1 1 1] Check If It's Time To Spawn Another
  (if (`self.Active`)
    (if (or (not (`KismetSystemLibrary.IsValid` _spawnedenemy)) (<= (`/Game/Blueprints/AI/AICharacter.Health` _spawnedenemy) 0.0))
      (if (> _spawntimer (`self.SecondsToNewSpawn`))
        (set `self.SpawnTimer` 0.0)
        ;[1 1 1] Destroy Old One If It Exists
        (`/Engine/EditorBlueprintResources/StandardMacros.IsValid` _spawnedenemy_2
          (:`Is Valid`
            (`self.K2_DestroyActor` _spawnedenemy_2))
          (:`Is Not Valid`
            _))
        ;[1 1 1] Spawn It
        (if (`KismetMathLibrary.RandomBool`)
          (bind _returnvalue_2 (`|SpawnActorFromClass` "/Game/Blueprints/AI/Enemies/LimeJellyAICharacter.LimeJellyAICharacter_C" _returnvalue))
          (bind _output_get (set `self.SpawnedEnemy` _returnvalue_2))
          ;[1 1 1] Add Monster To List. This Function Will Also Remove The Monster Furthest From The Player If There Are Too Many
          (`/Game/Blueprints/Monsters/BP_MonsterSpawnerControl.Add` _controller _output_get)
          (else
            (bind _returnvalue_3 (`|SpawnActorFromClass` "/Game/Blueprints/AI/Enemies/WhiplashAICharacter.WhiplashAICharacter_C" _returnvalue))
            (bind _output_get_2 (set `self.SpawnedEnemy` _returnvalue_3))
            (`/Game/Blueprints/Monsters/BP_MonsterSpawnerControl.Add` _controller _output_get_2)))
        (else
          (set `self.SpawnTimer` (+ _spawntimer (`GameplayStatics.GetWorldDeltaSeconds`))))))))

(event `self.Sphere.OnComponentBeginOverlap`
  (params (OtherActor :type "Actor Object Reference") (OtherComp :type "PrimitiveComponent Object Reference") (OtherBodyIndex :type Integer) (bFromSweep :type Boolean) (SweepResult :type "EngineTypes.HitResult Structure (by ref)"))
  ;[1 1 1] Keep Track Of If The Player Is Near
  (cast `/Game/Blueprints/DragonCharacter` OtherActor)
  (set `self.Active` true))

(event `self.Sphere.OnComponentEndOverlap`
  (params (OtherActor :type "Actor Object Reference") (OtherComp :type "PrimitiveComponent Object Reference") (OtherBodyIndex :type Integer))
  ;[1 1 1] Keep Track Of If The Player Is Near
  (cast `/Game/Blueprints/DragonCharacter` OtherActor)
  (set `self.Active` false))

(fn `UserConstructionScript`
  (bind _x (.x (`self.K2_GetActorLocation`)))
  (bind _y (.y (`self.K2_GetActorLocation`)))
  (bind _outhits (`KismetSystemLibrary.LineTraceMultiForObjects` (`KismetMathLibrary.MakeVector` _x _y 100000.0) (`KismetMathLibrary.MakeVector` _x _y -100000.0) (`|MakeArray` "ObjectTypeQuery1" :!type "EngineTypes.EObjectTypeQuery Enum")))
  (for _array_element _outhits
    (bind (_bblockinghit _time _location _normal _impactpoint _impactnormal _physmat _hitactor) (`GameplayStatics.BreakHitResult` _array_element))
    (cast `Landscape` _hitactor)
    (`self.K2_SetActorLocation` (+ _impactpoint (0.0 0.0 500.0)))))