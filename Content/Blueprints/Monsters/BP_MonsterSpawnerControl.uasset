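; BP_MonsterSpawnerControl tracks monsters in an array and culls them to limit how many exist in the world.
; On a timed Tick check, gated by a switch covering counts up to eleven, it destroys the first invalid, dead or too-distant monster.
; Add registers a monster and, above the cap, removes one chosen by a validity, health and player-distance scan, though its IsValid test matches every valid entry.
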(event EventBeginPlay)

(event EventActorBeginOverlap
  (params (OtherActor :type Actor%20Object%20Reference)))

(event EventTick
  (params (DeltaSeconds :type Float%20%28single-precision%29))
  (bind _monsters (Variables|Default|GetMonsters))
  (switch int (Utilities|Array|Length (Variables|Default|GetMonsters))
    (:0
      _)
    (:1
      _)
    (:2
      _)
    (:3
      _)
    (:4
      _)
    (:5
      _)
    (:6
      _)
    (:7
      _)
    (:8
      _)
    (:9
      _)
    (:10
      _)
    (:11
      _))
  (if (>= (Variables|Default|GetCheckTime) (Variables|Default|GetCheckInterval))
    (Variables|Default|SetCheckTime 0.0)
    (bind (_array_element _array_index) (Utilities|Array|ForEachLoopwithBreak _monsters :!label _label)
      (:LoopBody
        (if (Math|Boolean|ORBoolean (not (Utilities|IsValid _array_element)) (Variables|/Game/Blueprints/AI/AICharacter.AICharacter_C|GetDead _array_element) (>= (Transformation|GetHorizontalDistanceTo _array_element 0) (Variables|Default|GetMaxDistanceFromPlayer)))
          (Actor|DestroyActor _array_element)
          (Utilities|Array|RemoveIndex _monsters _array_index)
          (goto _label Break))))
    (else
      (Variables|Default|SetCheckTime (+ (Variables|Default|GetCheckTime) (Utilities|Time|GetWorldDeltaSeconds))))))

(fn ConstructionScript)

(fn Add
  (params (Monster :type AI%20Character%20Object%20Reference))
  (bind _returnvalue (Game|GetPlayerCharacter 0))
  (bind _monsters (Variables|Default|GetMonsters))
  (bind _returnvalue_2 (Transformation|GetHorizontalDistanceTo _returnvalue 0))
  (Utilities|Array|Add _monsters Monster)
  (if (> (Utilities|Array|Length _monsters) (Variables|Default|GetMaxNumberOfMonsters))
    ;[1 1 1] If there are too many monsters, remove the one that is furthest from the player, or any invalid indices or dead monsters found
    (bind (_array_element _array_index) (Utilities|Array|ForEachLoopwithBreak (Variables|Default|GetMonsters))
      (:LoopBody
        (if (Math|Boolean|ORBoolean (Utilities|IsValid _array_element) (< (Variables|/Game/Blueprints/AI/AICharacter.AICharacter_C|GetHealth _array_element) 0.0) (> _returnvalue_2 (Variables|Default|GetMaxDistanceFromPlayer)))
          (LocalVariables|SetLocalLongestIndex _array_index)
          (elif (> _returnvalue_2 (LocalVariables|GetLocalLongestLength))
            (LocalVariables|SetLocalLongestLength _returnvalue_2)
            (LocalVariables|SetLocalLongestIndex _array_index))))
      (:Completed
        (Utilities|IsValid (Utilities|Array|Get(acopy) (Variables|Default|GetMonsters) (LocalVariables|GetLocalLongestIndex))
          (:Is%20Valid
            (Actor|DestroyActor (Utilities|Array|Get(acopy) (Variables|Default|GetMonsters) (LocalVariables|GetLocalLongestIndex))))
          (:Is%20Not%20Valid
            _))
        (Utilities|Array|RemoveIndex (Variables|Default|GetMonsters) (LocalVariables|GetLocalLongestIndex))))))