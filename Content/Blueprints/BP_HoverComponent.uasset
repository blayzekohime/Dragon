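; BP_HoverComponent is a component that makes its owning actor hover above surfaces using physics.
; On initialize it caches the owner's first primitive component and enables physics simulation on it.
; Each tick it traces straight down from its location and, on a hit, applies force along the surface normal, fading linearly with distance, and sets linear and angular damping.
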(event `self.ReceiveTick`
  (params (DeltaSeconds :type "Float (single-precision)"))
  (bind _returnvalue (`self.K2_GetComponentLocation`))
  (bind (_outhit _returnvalue_2) (`KismetSystemLibrary.LineTraceSingle` _returnvalue (`KismetMathLibrary.MakeVector` (.x _returnvalue) (.y _returnvalue) (- (.z _returnvalue) (`self.TraceLength`))) "TraceTypeQuery1"))
  (if _returnvalue_2
    (bind (_bblockinghit _time _location _normal) (`GameplayStatics.BreakHitResult` _outhit))
    (`PrimitiveComponent.AddForce` (* _normal (`KismetMathLibrary.Lerp` (`self.HoverForce`) 0.0 (/ (`KismetMathLibrary.VSize` (- _location (`self.K2_GetComponentLocation`))) (`self.TraceLength`)))))
    (`PrimitiveComponent.SetLinearDamping` (`self.LinearDamping`))
    (`PrimitiveComponent.SetAngularDamping` (`self.AngularDamping`))))

(event `self.ReceiveInitializeComponent`
  ;[1 1 1] Initialize
  (bind _output_get (set `self.PrimitiveComponent` (`KismetArrayLibrary.Array_Get` (`Actor.K2_GetComponentsByClass` (`self.GetOwner`) "/Script/Engine.PrimitiveComponent"))))
  (`PrimitiveComponent.SetSimulatePhysics` _output_get true))