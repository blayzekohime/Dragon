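; BP_SonicAttack is a sonic attack projectile usable by both the player dragon and AI characters.
; Each tick it sweeps forward along the dragon's DropLocation, or along an AI instigator's right vector, and destroys itself after half a second.
; On overlap, IsPlayer selects the target: AI get a radial impulse and damage, while the dragon takes damage and is launched along the AI owner's forward vector.
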(event `self.ReceiveBeginPlay`)

(event `self.ReceiveActorBeginOverlap`
  (params (OtherActor :type "Actor Object Reference"))
  (bind _sonichealthdamage (`self.SonicHealthDamage`))
  (bind _sonicstaminadamage (`self.SonicStaminaDamage`))
  (bind _sonicbreathdamage (`self.SonicBreathDamage`))
  (if (`self.IsPlayer`)
    ;[1 1 1] Player hitting AI
    (bind _asaicharacter (cast `/Game/Blueprints/AI/AICharacter` OtherActor))
    (`/Engine/EditorBlueprintResources/StandardMacros.IsValid` _asaicharacter
      (:`Is Valid`
        (`PrimitiveComponent.AddRadialImpulse` _asaicharacter (`SceneComponent.K2_GetComponentLocation`) 1000.0 1000.0 "RIF_Constant" true)
        (`/Game/Blueprints/AI/AICharacter.Hurt` _asaicharacter _sonichealthdamage _sonicstaminadamage _sonicbreathdamage (`GameplayStatics.GetPlayerCharacter` 0))))
    (else
      ;[1 1 1] AI Hitting Player
      (bind _asdragon_character (cast `/Game/Blueprints/DragonCharacter` OtherActor))
      (`/Engine/EditorBlueprintResources/StandardMacros.IsValid` _asdragon_character
        (:`Is Valid`
          (`/Game/Blueprints/DragonCharacter.Hurt` _asdragon_character _sonichealthdamage _sonicstaminadamage _sonicbreathdamage)
          ;;[1 1 1] I think something wrong here
          (bind _asaicharacter_2 (cast `/Game/Blueprints/AI/AICharacter` (`self.GetOwner`)))
          (`/Engine/EditorBlueprintResources/StandardMacros.IsValid` _asaicharacter_2
            (:`Is Valid`
              (`Character.LaunchCharacter` _asdragon_character (* (`SceneComponent.GetForwardVector` _asaicharacter_2) 30000.0) true true))))))))

(event `self.ReceiveTick`
  (params (DeltaSeconds :type "Float (single-precision)"))
  (bind _returnvalue (`SceneComponent.K2_GetComponentLocation` self))
  ;[1 1 1] If Alive, Move it forward for a bit and then
  ; destroy after half a second
  (`/Engine/EditorBlueprintResources/StandardMacros.IsValid` self
    (:`Is Valid`
      (bind _asdragon_character (cast `/Game/Blueprints/DragonCharacter` (`self.GetInstigator` self))
        (:`then`
          (`self.K2_SetActorLocation` (+ (* (`SceneComponent.GetForwardVector` (`/Game/Blueprints/DragonCharacter.DropLocation` _asdragon_character)) 20.0) _returnvalue) true))
        (:`CastFailed`
          (bind _asaicharacter (cast `/Game/Blueprints/AI/AICharacter` (`self.GetInstigator` self)))
          (`self.K2_SetActorLocation` (+ (* (`SceneComponent.GetRightVector` _asaicharacter) 20.0) _returnvalue) true)))
      (`KismetSystemLibrary.Delay` 0.5)
      (`self.K2_DestroyActor`))))

(fn `UserConstructionScript`)