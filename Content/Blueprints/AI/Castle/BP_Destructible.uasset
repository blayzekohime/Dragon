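; Destructible castle piece with soak-reduced health that the player dragon can destroy and that can be repaired until destroyed.
; Five collision boxes catch ranged and sonic hits and track dragon overlap, letting Tick apply breath damage over time.
; At zero health it disables collision, removes nearby navigation BlockingVolumes, clears itself from targeting and hurts units guarding or repairing it.
; Tick also billboards and scales a visible target marker from the mesh bounds.
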(event OnComponentBeginOverlap(CollisionMain)
  (params (OtherActor :type Actor%20Object%20Reference) (OtherComp :type Primitive%20Component%20Object%20Reference) (OtherBodyIndex :type Integer) (bFromSweep :type Boolean) (SweepResult :type Hit%20Result%20Structure%20%28by%20ref%29))
  ;[1 1 1] Keep Track Of Collisions
  (bind _collidingwithplayer (CallFunction|StartOverlap OtherActor))
  (bind _output_get (Variables|Default|SetPlayerCollidingWithMain _collidingwithplayer))
  (Variables|Default|SetPlayerColliding _output_get))

(event OnComponentEndOverlap(CollisionMain)
  (params (OtherActor :type Actor%20Object%20Reference) (OtherComp :type Primitive%20Component%20Object%20Reference) (OtherBodyIndex :type Integer))
  ;[1 1 1] Keep Track Of Collisions
  (bind _wasplayer (CallFunction|EndOverlap OtherActor))
  (if _wasplayer
    (Variables|Default|SetPlayerCollidingWithMain false)
    (Variables|Default|SetPlayerColliding (Math|Boolean|ORBoolean (Variables|Default|GetPlayerCollidingWithMain) (Variables|Default|GetPlayerCollidingWithEdge1) (Variables|Default|GetPlayerCollidingWithEdge2) (Variables|Default|GetPlayerCollidingWithEdge3) (Variables|Default|GetPlayerCollidingWithEdge4)))))

(event OnComponentBeginOverlap(CollisionEdge1)
  (params (OtherActor :type Actor%20Object%20Reference) (OtherComp :type Primitive%20Component%20Object%20Reference) (OtherBodyIndex :type Integer) (bFromSweep :type Boolean) (SweepResult :type Hit%20Result%20Structure%20%28by%20ref%29))
  ;[1 1 1] Keep Track Of Collisions
  (bind _collidingwithplayer (CallFunction|StartOverlap OtherActor))
  (bind _output_get (Variables|Default|SetPlayerCollidingWithEdge1 _collidingwithplayer))
  (Variables|Default|SetPlayerColliding _output_get))

(event OnComponentEndOverlap(CollisionEdge1)
  (params (OtherActor :type Actor%20Object%20Reference) (OtherComp :type Primitive%20Component%20Object%20Reference) (OtherBodyIndex :type Integer))
  ;[1 1 1] Keep Track Of Collisions
  (bind _wasplayer (CallFunction|EndOverlap OtherActor))
  (if _wasplayer
    (Variables|Default|SetPlayerCollidingWithEdge1 false)
    (Variables|Default|SetPlayerColliding (Math|Boolean|ORBoolean (Variables|Default|GetPlayerCollidingWithMain) (Variables|Default|GetPlayerCollidingWithEdge1) (Variables|Default|GetPlayerCollidingWithEdge2) (Variables|Default|GetPlayerCollidingWithEdge3) (Variables|Default|GetPlayerCollidingWithEdge4)))))

(event OnComponentBeginOverlap(CollisionEdge2)
  (params (OtherActor :type Actor%20Object%20Reference) (OtherComp :type Primitive%20Component%20Object%20Reference) (OtherBodyIndex :type Integer) (bFromSweep :type Boolean) (SweepResult :type Hit%20Result%20Structure%20%28by%20ref%29))
  ;[1 1 1] Keep Track Of Collisions
  (bind _collidingwithplayer (CallFunction|StartOverlap OtherActor))
  (bind _output_get (Variables|Default|SetPlayerCollidingWithEdge2 _collidingwithplayer))
  (Variables|Default|SetPlayerColliding _output_get))

(event OnComponentEndOverlap(CollisionEdge2)
  (params (OtherActor :type Actor%20Object%20Reference) (OtherComp :type Primitive%20Component%20Object%20Reference) (OtherBodyIndex :type Integer))
  ;[1 1 1] Keep Track Of Collisions
  (bind _wasplayer (CallFunction|EndOverlap OtherActor))
  (if _wasplayer
    (Variables|Default|SetPlayerCollidingWithEdge2 false)
    (Variables|Default|SetPlayerColliding (Math|Boolean|ORBoolean (Variables|Default|GetPlayerCollidingWithMain) (Variables|Default|GetPlayerCollidingWithEdge1) (Variables|Default|GetPlayerCollidingWithEdge2) (Variables|Default|GetPlayerCollidingWithEdge3) (Variables|Default|GetPlayerCollidingWithEdge4)))))

(event OnComponentBeginOverlap(CollisionEdge3)
  (params (OtherActor :type Actor%20Object%20Reference) (OtherComp :type Primitive%20Component%20Object%20Reference) (OtherBodyIndex :type Integer) (bFromSweep :type Boolean) (SweepResult :type Hit%20Result%20Structure%20%28by%20ref%29))
  ;[1 1 1] Keep Track Of Collisions
  (bind _collidingwithplayer (CallFunction|StartOverlap OtherActor))
  (bind _output_get (Variables|Default|SetPlayerCollidingWithEdge3 _collidingwithplayer))
  (Variables|Default|SetPlayerColliding _output_get))

(event OnComponentEndOverlap(CollisionEdge3)
  (params (OtherActor :type Actor%20Object%20Reference) (OtherComp :type Primitive%20Component%20Object%20Reference) (OtherBodyIndex :type Integer))
  ;[1 1 1] Keep Track Of Collisions
  (bind _wasplayer (CallFunction|EndOverlap OtherActor))
  (if _wasplayer
    (Variables|Default|SetPlayerCollidingWithEdge3 false)
    (Variables|Default|SetPlayerColliding (Math|Boolean|ORBoolean (Variables|Default|GetPlayerCollidingWithMain) (Variables|Default|GetPlayerCollidingWithEdge1) (Variables|Default|GetPlayerCollidingWithEdge2) (Variables|Default|GetPlayerCollidingWithEdge3) (Variables|Default|GetPlayerCollidingWithEdge4)))))

(event OnComponentBeginOverlap(CollisionEdge4)
  (params (OtherActor :type Actor%20Object%20Reference) (OtherComp :type Primitive%20Component%20Object%20Reference) (OtherBodyIndex :type Integer) (bFromSweep :type Boolean) (SweepResult :type Hit%20Result%20Structure%20%28by%20ref%29))
  ;[1 1 1] Keep Track Of Collisions
  (bind _collidingwithplayer (CallFunction|StartOverlap OtherActor))
  (bind _output_get (Variables|Default|SetPlayerCollidingWithEdge4 _collidingwithplayer))
  (Variables|Default|SetPlayerColliding _output_get))

(event OnComponentEndOverlap(CollisionEdge4)
  (params (OtherActor :type Actor%20Object%20Reference) (OtherComp :type Primitive%20Component%20Object%20Reference) (OtherBodyIndex :type Integer))
  ;[1 1 1] Keep Track Of Collisions
  (bind _wasplayer (CallFunction|EndOverlap OtherActor))
  (if _wasplayer
    (Variables|Default|SetPlayerCollidingWithEdge4 false)
    (Variables|Default|SetPlayerColliding (Math|Boolean|ORBoolean (Variables|Default|GetPlayerCollidingWithMain) (Variables|Default|GetPlayerCollidingWithEdge1) (Variables|Default|GetPlayerCollidingWithEdge2) (Variables|Default|GetPlayerCollidingWithEdge3) (Variables|Default|GetPlayerCollidingWithEdge4)))))

(event EventTick
  (params (DeltaSeconds :type Float%20%28single-precision%29))
  (bind _returnvalue (Game|GetPlayerCameraManager 0))
  (bind _uitarget (Variables|Default|GetUITarget))
  (bind _destructiblecomponent (Variables|Default|GetDestructibleComponent))
  (bind _destructiblecomponent_2 (Variables|Default|GetDestructibleComponent))
  (bind (_origin _boxextent) (Collision|GetComponentBounds _destructiblecomponent))
  (bind _returnvalue_2 (Transformation|GetWorldLocation _destructiblecomponent_2))
  (bind _returnvalue_3 (Camera|GetCameraLocation _returnvalue))
  (bind (_x _y _z) (Math|Vector|BreakVector _boxextent))
  (bind _returnvalue_4 (Math|Rotator|FindLookatRotation _returnvalue_2 _returnvalue_3))
  (bind (_pitch _yaw _roll) (Class|KismetMathLibrary|BreakRot _returnvalue_4))
  (bind _returnvalue_5 (Math|Float|Max(Float) _x _y _z))
  ;[1 1 1] Only Position Target If It Is Visible
  (if (Variables|/Script/Engine.SceneComponent|GetbVisible (Variables|Default|GetUITarget))
    ;[1 1 1] Position Target
    (Transformation|SetWorldLocation _uitarget (+ _origin (* (Class|KismetMathLibrary|GetDirectionVector _origin _returnvalue_3) (* _returnvalue_5 2.0))) false)
    (Transformation|SetWorldRotation _uitarget (Class|KismetMathLibrary|MakeRot (+ _pitch -9e+01) _yaw _roll) false)
    (Transformation|SetWorldScale3D _uitarget (Math|Conversions|ToVector(Float) (* _returnvalue_5 0.0075))))
  ;[1 1 1] Take Damage When Colliding With An Active Player Breath Weapon
  (if (Variables|Default|GetPlayerColliding)
    (bind _asdragon_character (Utilities|Casting|CastToDragonCharacter (Game|GetPlayerCharacter 0)))
    (if (Variables|/Game/Blueprints/DragonCharacter.DragonCharacter_C|GetIsBreathing _asdragon_character)
      (for _array_element (Class|PrimitiveComponent|GetOverlappingComponents)
        (bind _asbox_collision (Utilities|Casting|CastToBoxComponent _array_element))
        (if (== _asbox_collision (Variables|/Game/Blueprints/DragonCharacter.DragonCharacter_C|GetBreathCollision _asdragon_character))
          (CallFunction|Damage (* (Utilities|Time|GetWorldDeltaSeconds) (Variables|/Game/Blueprints/DragonCharacter.DragonCharacter_C|GetBreathDamage _asdragon_character)) (.Origin (Collision|GetComponentBounds 0)) "0, 0, 0" 1e+03))))))

(fn ConstructionScript
  (bind _returnvalue (Transformation|GetWorldLocation))
  (Transformation|SetWorldLocation (+ (Variables|Default|GetGuardPoint) _returnvalue) false)
  (Transformation|SetWorldLocation (+ (Variables|Default|GetRepairPointLocation1) _returnvalue) false)
  (Transformation|SetWorldLocation (Variables|Default|GetRepairPointLocation2) false))

(fn Damage
  (params (DamageAmount :type Float%20%28single-precision%29 :default 0.0) (HitLocation :type Vector :default "0, 0, 0") (ImpulseDir :type Vector :default "0, 0, 0") (ImpulseStregith :type Float%20%28single-precision%29 :default 0.0))
  (bind _soak (Variables|Default|GetSoak))
  (bind _returnvalue (- 1.0 _soak))
  (bind _returnvalue_2 (* DamageAmount _returnvalue))
  ;[1 1 1] Damage
  (Game|Damage|ApplyDamage _returnvalue_2 HitLocation ImpulseDir ImpulseStregith)
  ;[1 1 1] Destroy
  (bind _output_get (Variables|Default|SetHealth (- (Variables|Default|GetHealth) _returnvalue_2)))
  (if (<= _output_get 0.0)
    (Utilities|FlowControl|Sequence
      (:then_0
        ;[1 1 1] Be Sure
        (Utilities|FlowControl|DoOnce false
          (:Completed
            (Game|Damage|ApplyDamage (Variables|Default|GetDestructibleComponent) 5.0 HitLocation ImpulseDir ImpulseStregith)
            ;[1 1 1] Disable collision boxes
            (Collision|SetCollisionEnabled (Variables|Default|GetCollisionMain) "NoCollision")
            ;[1 1 1] Destroy Blocking Volume I had To Get Navigation To Pay Attention To The Destructibles
            (bind _outactors (Actor|GetAllActorsOfClass "/Script/Engine.BlockingVolume"))
            (for _array_element _outactors
              (Utilities|IsValid _array_element
                (:Is%20Valid
                  (if (< (Transformation|GetHorizontalDistanceTo _array_element) 2e+02)
                    (Actor|DestroyActor _array_element))))))))
      (:then_1
        (Variables|Default|SetDestroyed true)
        (bind _asdragon_character (Utilities|Casting|CastToDragonCharacter (Game|GetPlayerCharacter 0)))
        (Default|RemoveKilledTarget (Variables|/Game/Blueprints/DragonCharacter.DragonCharacter_C|GetBP_Targeting _asdragon_character) self)
        ;[1 1 1] Damage Any Units Guarding Or Repairing It
        (if (Variables|Default|GetGuarded)
          (Default|Hurt (Variables|Default|GetGuardingMe) (Variables|Default|GetDestructionDamage) 0.0 0.0 (Game|GetPlayerCharacter 0))
          (Variables|Default|SetGuarded false))
        (if (Variables|Default|GetBeingRepaired)
          (Default|Hurt (Variables|Default|GetRepairingMe) (Variables|Default|GetDestructionDamage) 0.0 0.0 (Game|GetPlayerCharacter 0)))))))

(fn Fix
  (params (FixAmount :type Float%20%28single-precision%29 :default 0.0))
  (if (> (Variables|Default|GetHealth) 0.0)
    (Variables|Default|SetHealth (Math|Float|Min(Float) (+ (Variables|Default|GetHealth) FixAmount) 1.0))))

(fn StartOverlap
  (params (OtherActor :type Actor%20Object%20Reference))
  (if (Variables|Default|GetDestroyed)
    (LocalVariables|SetOutputCollidingWithPlayer false :!label _label)
    (return (LocalVariables|GetOutputCollidingWithPlayer))
    (else
      (bind _asbp_ranged_attack (Utilities|Casting|CastToBP_RangedAttack OtherActor)
        (:then
          (Utilities|IsValid _asbp_ranged_attack
            (:Is%20Valid
              (if (!= _asbp_ranged_attack (Variables|Default|GetLastRangedStrike))
                (Variables|Default|SetLastRangedStrike _asbp_ranged_attack)
                (bind _isplayers (Default|GetIsPlayers _asbp_ranged_attack))
                (if _isplayers
                  (CallFunction|Damage (Variables|/Game/Blueprints/BP_RangedAttack.BP_RangedAttack_C|GetDamageHealth _asbp_ranged_attack) (Transformation|GetActorLocation _asbp_ranged_attack) (Class|KismetMathLibrary|GetDirectionVector (Transformation|GetActorLocation _asbp_ranged_attack) (Transformation|GetActorLocation)) 1e+06)
                  (Default|Explode _asbp_ranged_attack)
                  (goto _label))))))
        (:CastFailed
          (bind _asdragon_character (Utilities|Casting|CastToDragonCharacter OtherActor)
            (:then
              (Utilities|IsValid _asdragon_character
                (:Is%20Valid
                  (LocalVariables|SetOutputCollidingWithPlayer true)
                  (return (LocalVariables|GetOutputCollidingWithPlayer)))))
            (:CastFailed
              (bind _asbp_sonic_attack (Utilities|Casting|CastToBP_SonicAttack OtherActor))
              (Utilities|IsValid _asbp_sonic_attack
                (:Is%20Valid
                  (if (!= _asbp_sonic_attack (Variables|Default|GetLastSonicStrike))
                    (Variables|Default|SetLastSonicStrike _asbp_sonic_attack)
                    (CallFunction|Damage (Variables|/Game/Blueprints/BP_SonicAttack.BP_SonicAttack_C|GetSonicHealthDamage _asbp_sonic_attack) (Transformation|GetActorLocation _asbp_sonic_attack) (Class|KismetMathLibrary|GetDirectionVector (Transformation|GetActorLocation _asbp_sonic_attack) (Transformation|GetActorLocation)) 1e+06)
                    (goto _label)))))))))))

(fn EndOverlap
  (params (OtherActor :type Actor%20Object%20Reference))
  (bind _asdragon_character (Utilities|Casting|CastToDragonCharacter OtherActor)
    (:then
      (Utilities|IsValid _asdragon_character
        (:Is%20Valid
          (LocalVariables|SetOutputWasPlayer true))
        (:Is%20Not%20Valid
          (LocalVariables|SetOutputWasPlayer false :!label _label))))
    (:CastFailed
      (goto _label)))
  (return (LocalVariables|GetOutputWasPlayer)))