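; AI controller that runs a behavior tree and manages when an AI character chases or flees from the player.
; Perception updates containing a DragonCharacter set the CanSeePlayer blackboard key and raise the pawn's walk speed to its run speed.
; A throttled Tick clears that key once the player is beyond StopChasingRange, unless the player has injured the AI.
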(event `self.ReceiveTick`
  (params (DeltaSeconds :type "Float (single-precision)"))
  (bind _returnvalue (`self.K2_GetPawn`))
  ;[1 0 1] Event Tick
  ;;[1 1 1] Only Refresh This Every TickEveryXSeconds Seconds
  (if (>= (+ (`self.TimeSinceLastCheck`) DeltaSeconds) (`self.TickEveryXSeconds`))
    (set `self.TimeSinceLastCheck` 0.0)
    ;;[1 1 1] Only Proceed If Player Has Been Spotted
    (if (`BlackboardComponent.GetValueAsBool` (`AIBlueprintHelperLibrary.GetBlackboard` self) "CanSeePlayer")
      ;;[1 1 1] If Has Been Injured By Player, Never Stop
      (bind _asaicharacter (cast `/Game/Blueprints/AI/AICharacter` _returnvalue))
      ;;[1 1 1] Check If Player Has Gone Outside Of Sight Range
      (if (not (or (`/Game/Blueprints/AI/AICharacter.InjuredByPlayer` _asaicharacter) (<= (`self.GetDistanceTo` _returnvalue (`GameplayStatics.GetPlayerCharacter` 0)) (`/Game/Blueprints/AI/AICharacter.StopChasingRange` _asaicharacter))))
        ;;[1 1 1] If They Have Gone Out Of Range, Stop Chasing
        (`BlackboardComponent.SetValueAsBool` (`AIBlueprintHelperLibrary.GetBlackboard` self) "CanSeePlayer" false)))))

(event `self.ReceiveBeginPlay`
  ;[1 1 1] Set Behavior Tree
  (`self.RunBehaviorTree` "/Game/Blueprints/AI/AIBehaviorTree.AIBehaviorTree"))

(event `self.AIPerception.OnPerceptionUpdated`
  (params (UpdatedActors :type "Array of Actor Object Reference"))
  ;[1 0 1] When It Sees The Character
  ;;[1 1 1] Get List Of Actors It Can See
  (for _array_element UpdatedActors
    ;;[1 1 1] Tell Behavior Tree That Player Is Seen
    (cast `/Game/Blueprints/DragonCharacter` _array_element)
    (`BlackboardComponent.SetValueAsBool` (`AIBlueprintHelperLibrary.GetBlackboard` self) "CanSeePlayer" true)
    ;;[1 1 1] Speed Up To Chase (Or Flee)
    (bind _asaicharacter (cast `/Game/Blueprints/AI/AICharacter` (`self.K2_GetPawn`)))
    (set `CharacterMovementComponent.MaxWalkSpeed` (`/Game/Blueprints/AI/AICharacter.SpeedRun` _asaicharacter) (`Character.CharacterMovement` _asaicharacter))))

(fn `UserConstructionScript`)