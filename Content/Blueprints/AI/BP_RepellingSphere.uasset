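; BP_RepellingSphere is a spherical volume that pushes overlapping Characters away from its center.
; Each tick it filters Characters by flying, falling or walking state against per-mode toggles, then adds an outward force through CharacterMovement.
; The force blends from a center value to an edge value by distance over Radius, scaled by delta time.
; The construction script sizes the sphere component from Radius.
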(event `self.ReceiveTick`
  (params (DeltaSeconds :type "Float (single-precision)"))
  (bind _returnvalue (`SceneComponent.K2_GetComponentLocation` (`self.Sphere`)))
  (for _array_element (`PrimitiveComponent.GetOverlappingActors` "/Script/Engine.Character")
    (bind _ascharacter (cast `Character` _array_element))
    (if (or (and (`NavMovementComponent.IsFlying` _ascharacter) (`self.RepelFlyers`)) (and (`NavMovementComponent.IsFalling` _ascharacter) (`self.RepelFallers`)) (and (`CharacterMovementComponent.IsWalking` _ascharacter) (`self.RepelWalkers`)))
      (bind _returnvalue_2 (`self.K2_GetActorLocation` _ascharacter))
      (`CharacterMovementComponent.AddForce` (`Character.CharacterMovement` _ascharacter) (* (`KismetMathLibrary.GetDirectionVector` _returnvalue _returnvalue_2) (* (`GameplayStatics.GetWorldDeltaSeconds`) (`KismetMathLibrary.Lerp` (`self.ForceAtCenter`) (`self.ForceAtEdge`) (/ (`KismetMathLibrary.VSize` (- _returnvalue _returnvalue_2)) (`self.Radius`)))))))))

(fn `UserConstructionScript`
  (`SphereComponent.SetSphereRadius` (`self.Radius`)))